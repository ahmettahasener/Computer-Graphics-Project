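; BP_Target is a collectible target that jumps to a new spot and adds to a score when touched.
; On BeginPlay it caches every TargetPoint in the level.
; Any actor overlapping its Box teleports it to a random cached point, raises its own Score variable and prints a pickup message.
; The OffroadCar_Pawn cast and ScoreText widget creation are unconnected, so overlaps are unfiltered and that widget never appears.
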(event `self.ReceiveBeginPlay`
  (bind _outactors (`GameplayStatics.GetAllActorsOfClass` "/Script/Engine.TargetPoint"))
  (set `self.Positions` _outactors))

(event `self.Box.OnComponentBeginOverlap`
  (params (OverlappedComponent :type "PrimitiveComponent Object Reference") (OtherActor :type "Actor Object Reference") (OtherComp :type "PrimitiveComponent Object Reference") (OtherBodyIndex :type Integer) (bFromSweep :type Boolean) (SweepResult :type "HitResult Structure (by ref)"))
  (`self.K2_SetActorLocation` (`self.K2_GetActorLocation` (`|GetArrayItem` (`self.Positions`) (`KismetMathLibrary.RandomIntegerInRange` 0 (- (`KismetArrayLibrary.Array_Length` (`self.Positions`)) 1)))))
  (set `self.Score` (+ (`self.Score`) 10))
  (`KismetSystemLibrary.PrintText` "Target Collected !" true false (struct :`R` 1.0 :`B` 0.898733 :`A` 1.0) 5.0))

(fn `UserConstructionScript`)